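; BP_GameLetterSLot is a letter slot actor for a word game, showing one letter of a three-letter word on its PhysicalLetter text.
; On BeginPlay it builds a hard-coded word struct array and resets ActiveId to 0.
; GetLetter clears the text and caches the active word's letters; after a delay SetLetter shows the one matching SlotPosition, repeating on any overlap.
; CollisionDetected is an uncalled stub whose letter comparisons do nothing.
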(event EventBeginPlay
  ;[1 1 1] Comment
  (CallFunction|CreateWordArray)
  (Utilities|FlowControl|Delay 2.0)
  (CallFunction|GetLetter)
  (Utilities|FlowControl|Delay 2.0)
  (CallFunction|SetLetter))

(event Collision|EventActorBeginOverlap
  (params (OtherActor :type Actor%20Object%20Reference))
  ;[1 1 1] Comment
  (CallFunction|GetLetter)
  (Utilities|FlowControl|Delay 2.0)
  (CallFunction|SetLetter))

(event EventTick
  (params (DeltaSeconds :type Float%20%28single-precision%29)))

(fn ConstructionScript)

(fn GetLetter
  (Utilities|Casting|CastToThirdPersonCharacter (Game|Player|GetPlayerPawn 0)
    (:then
      (Development|PrintString "Cast 3PC Go" false true "(R=0.313989,G=0.871367,B=0.061246,A=1.000000)")
      (Development|PrintString "GL: Test Clear Billboard" false true "(R=1.000000,G=0.020833,B=0.039864,A=1.000000)" 5.0)
      (Rendering|Components|TextRender|SetText (Variables|Default|GetPhysicalLetter) (Class|KismetTextLibrary|GetEmptyText))
      (for (_array_element _array_index) (Variables|Default|GetArrayOfGameWords)
        (Development|PrintString "GL: Loop Start" false true "(R=0.871367,G=0.238398,B=0.059511,A=1.000000)")
        (if (== (Variables|Default|GetActiveId) _array_index)
          (Development|PrintString (.GW_word (Utilities|Struct|BreakStruct_GameWords _array_element)) false true "(R=0.871367,G=0.859233,B=0.134450,A=1.000000)")
          (Variables|Default|SetGWLetterOne (Utilities|Text|ToText(String) (.GW_letter_1 (Utilities|Struct|BreakStruct_GameWords _array_element))))
          (Variables|Default|SetGWLetterTwo (Utilities|Text|ToText(String) (.GW_letter_2 (Utilities|Struct|BreakStruct_GameWords _array_element))))
          (Variables|Default|SetGWLetterThree (Utilities|Text|ToText(String) (.GW_letter_3 (Utilities|Struct|BreakStruct_GameWords _array_element))))
          (Development|PrintString "Finished Letter Set" false true "(R=0.871367,G=0.238398,B=0.059511,A=1.000000)")))
      (Development|PrintString "GL: Loop End" false true "(R=0.871367,G=0.238398,B=0.059511,A=1.000000)"))
    (:CastFailed
      (Development|PrintString "3PC Failed" false true "(R=1.000000,G=0.020833,B=0.039864,A=1.000000)"))))

(fn CreateWordArray
  (Variables|Default|SetActiveId 0)
  (Development|PrintString "Create Word Array" false true "(R=1.000000,G=0.138293,B=0.306577,A=1.000000)")
  (Variables|Default|SetArrayOfGameWords (Utilities|Array|MakeArray (Utilities|Struct|MakeStruct_GameWords (Variables|Default|GetActiveId) false) (Utilities|Struct|MakeStruct_GameWords (+ (Variables|Default|GetActiveId) 1) false 3 "COB" "C" "O" "B") (Utilities|Struct|MakeStruct_GameWords (+ (Variables|Default|GetActiveId) 1) false 3 "AND" "A" "N" "D")))
  (Development|PrintString "CWA: Start Loop" false true "(R=1.000000,G=0.138293,B=0.306577,A=1.000000)")
  (for _array_element (Variables|Default|GetArrayOfGameWords)
    (Development|PrintString (.GW_word (Utilities|Struct|BreakStruct_GameWords _array_element)) false true "(R=1.000000,G=0.138293,B=0.306577,A=1.000000)" 1e+01))
  (Development|PrintString "CWA: End Loop" false true "(R=1.000000,G=0.138293,B=0.306577,A=1.000000)"))

(fn SetLetter
  (Development|PrintString "Set Letter: " false true "(R=0.375104,G=0.032356,B=0.429167,A=1.000000)" 1e+01)
  (if (== (Variables|Default|GetSlotPosition) 1)
    (Rendering|Components|TextRender|SetText (Variables|Default|GetPhysicalLetter) (Variables|Default|GetGWLetterOne))
    (elif (== (Variables|Default|GetSlotPosition) 2)
      (Rendering|Components|TextRender|SetText (Variables|Default|GetPhysicalLetter) (Variables|Default|GetGWLetterTwo))
      (elif (== (Variables|Default|GetSlotPosition) 3)
        (Rendering|Components|TextRender|SetText (Variables|Default|GetPhysicalLetter) (Variables|Default|GetGWLetterThree))))))

(fn CollisionDetected
  (bind _physicalletter (Variables|Default|GetPhysicalLetter))
  (bind _returnvalue (Utilities|Text|ToText(Object) _physicalletter))
  (if (== (Variables|Default|GetSlotPosition) 1)
    (Development|PrintString (Utilities|String|ToString(Text) _returnvalue) true true "(R=0.000000,G=0.660000,B=1.000000,A=1.000000)" 1e+01)
    (if (Utilities|Enum|Equal(Enum) _returnvalue (Variables|Default|GetTest%20Variable))
      _)
    (elif (== (Variables|Default|GetSlotPosition) 2)
      (if (Utilities|Enum|Equal(Enum) (Utilities|Text|ToText(Object) (Variables|Default|GetPhysicalLetter)) (Variables|Default|GetGWLetterTwo))
        _)
      (elif (== (Variables|Default|GetSlotPosition) 3)
        (if (Utilities|Enum|Equal(Enum) (Utilities|Text|ToText(Object) (Variables|Default|GetPhysicalLetter)) (Variables|Default|GetGWLetterThree))
          _)))))