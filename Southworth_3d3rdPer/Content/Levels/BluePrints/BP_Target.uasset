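; BP_Target is a word-game target that shows one letter, or the whole word, of the current word according to its slot position.
; It builds hardcoded word and vowel arrays at BeginPlay, then sets its text, switching visibility for vowels.
; An overlapping BP_FlamingLetters with the matching letter is destroyed and adds points to the player's score.
; The hit fires an event dispatcher that advances and reloads every BP_Target to the next word.
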(event Custom|Event_updateAllTargets
  (CallFunction|UpdateTarget))

(event EventBeginPlay
  (Utilities|FlowControl|Sequence
    (:then_0
      (bind _asthird_person_character (Utilities|Casting|CastToThirdPersonCharacter (Game|GetPlayerCharacter 0)))
      (Variables|Default|SetCharacterReference _asthird_person_character))
    (:then_1
      (CallFunction|CreateWords))
    (:then_2
      (CallFunction|CreateVowels))
    (:then_3
      (Utilities|FlowControl|Delay 0.5)
      (CallFunction|LoadLetters))
    (:then_4
      (EventDispatchers|BindEventtoUpdateAllTargets (delegate Custom|Event_updateAllTargets)))))

(event Collision|EventActorBeginOverlap
  (params (OtherActor :type Actor%20Object%20Reference))
  ;[1 1 1] Comment
  (bind _asbp_flaming_letters (Utilities|Casting|CastToBP_FlamingLetters OtherActor))
  (if (Utilities|Enum|Equal(Enum) (Variables|Default|GetCurrentLetter) (Variables|/Game/Levels/BluePrints/BP_FlamingLetters.BP_FlamingLetters_C|GetBP_FL_txtLetter _asbp_flaming_letters))
    (Development|PrintString "Letter is: ")
    (Development|PrintString "Hello")
    (CallFunction|SuccessPoint)
    (Actor|DestroyActor OtherActor)
    (Default|CallUpdateAllTargets)))

(event EventTick
  (params (DeltaSeconds :type Float%20%28single-precision%29)))

(fn ConstructionScript)

(fn LoadLetters
  (bind _slotposition (Variables|Default|GetSlotPosition))
  (bind _targetletter (Variables|Default|GetTargetLetter))
  (Development|PrintString "Load Letter" false false "(R=0.000000,G=0.660000,B=1.000000,A=1.000000)" 5.0)
  (bind _array_element (Utilities|Array|ForEachLoopwithBreak (Variables|Default|GetTargetArray))
    (:LoopBody
      (if (== (Variables|Default|GetCurrentWord) (.Target_ID (Utilities|Struct|BreakTargetStruct _array_element)))
        (if (== _slotposition 1)
          (Rendering|Components|TextRender|SetText _targetletter (.Target_Letter_1 (Utilities|Struct|BreakTargetStruct _array_element)))
          (Variables|Default|SetCurrentLetter (.Target_Letter_1 (Utilities|Struct|BreakTargetStruct _array_element)))
          (Rendering|SetVisibility (Variables|Default|GetTargetLetter) (Variables|Default|GetVisibleOn) false :!label _label)
          (bind _array_element_2 (Utilities|Array|ForEachLoopwithBreak (Variables|Default|GetVowelArray))
            (:LoopBody
              (if (Utilities|Enum|Equal(Enum) (Variables|Default|GetCurrentLetter) (.txtVowel (Utilities|Struct|BreakVowelStructure _array_element_2)))
                (Rendering|SetVisibility (Variables|Default|GetTargetLetter) (Variables|Default|GetVisibleOff) false))))
          (elif (== _slotposition 2)
            (Rendering|Components|TextRender|SetText _targetletter (.Target_Letter_2 (Utilities|Struct|BreakTargetStruct _array_element)))
            (Variables|Default|SetCurrentLetter (.Target_Letter_2 (Utilities|Struct|BreakTargetStruct _array_element)))
            (goto _label)
            (elif (== _slotposition 3)
              (Rendering|Components|TextRender|SetText _targetletter (.Target_Letter_3 (Utilities|Struct|BreakTargetStruct _array_element)))
              (Variables|Default|SetCurrentLetter (.Target_Letter_3 (Utilities|Struct|BreakTargetStruct _array_element)))
              (goto _label)
              (elif (== _slotposition 4)
                (Rendering|Components|TextRender|SetText _targetletter (.Target_Word (Utilities|Struct|BreakTargetStruct _array_element)))
                (Variables|Default|SetCurrentLetter (.Target_Word (Utilities|Struct|BreakTargetStruct _array_element)))
                (goto _label)))))))))

(fn CreateWords
  (Utilities|FlowControl|DoOnce false
    (:Completed
      (bind _structout (Utilities|Struct|SetmembersinTargetStruct (Utilities|Struct|MakeTargetStruct 0 true 3 10 "BIT" "B" "I" "T")))
      (bind _structout_2 (Utilities|Struct|SetmembersinTargetStruct (Utilities|Struct|MakeTargetStruct 1 true 3 10 "MEN" "M" "E" "N")))
      (bind _structout_3 (Utilities|Struct|SetmembersinTargetStruct (Utilities|Struct|MakeTargetStruct 2 true 3 10 "AND" "A" "N" "D")))
      (Variables|Default|SetTargetArray (Utilities|Array|MakeArray _structout _structout_2 _structout_3))
      (for _array_element (Utilities|Array|MakeArray _structout _structout_2 _structout_3)
        (Development|PrintString (Utilities|String|ToString(Text) (.Target_Word (Utilities|Struct|BreakTargetStruct _array_element))) false)))))

(fn ChangeWord
  (Variables|Default|SetCurrentWord (+ (Variables|Default|GetCurrentWord) 1)))

(fn CreateVowels
  (bind _structout (Utilities|Struct|SetmembersinVowelStructure (Utilities|Struct|MakeVowelStructure 0 "A" "A")))
  (bind _structout_2 (Utilities|Struct|SetmembersinVowelStructure (Utilities|Struct|MakeVowelStructure 0 "E" "E")))
  (bind _structout_3 (Utilities|Struct|SetmembersinVowelStructure (Utilities|Struct|MakeVowelStructure 0 "I" "I")))
  (bind _structout_4 (Utilities|Struct|SetmembersinVowelStructure (Utilities|Struct|MakeVowelStructure 0 "O" "O")))
  (bind _structout_5 (Utilities|Struct|SetmembersinVowelStructure (Utilities|Struct|MakeVowelStructure 0 "U" "U")))
  (bind _structout_6 (Utilities|Struct|SetmembersinVowelStructure (Utilities|Struct|MakeVowelStructure 0 "Y" "Y")))
  (Variables|Default|SetVowelArray (Utilities|Array|MakeArray _structout _structout_2 _structout_3 _structout_4 _structout_5 _structout_6)))

(fn SuccessPoint
  (bind _characterreference (Variables|Default|GetCharacterReference))
  (bind _output_get (Variables|/Game/ThirdPersonBP/Blueprints/ThirdPersonCharacter.ThirdPersonCharacter_C|SetPlayerScore _characterreference (+ (Variables|/Game/ThirdPersonBP/Blueprints/ThirdPersonCharacter.ThirdPersonCharacter_C|GetPointValue _characterreference) (Variables|/Game/ThirdPersonBP/Blueprints/ThirdPersonCharacter.ThirdPersonCharacter_C|GetPlayerScore _characterreference))))
  (Development|PrintString "Score: ")
  (Development|PrintString (Utilities|String|ToString(Integer) _output_get)))

(fn UpdateTarget
  (bind _outactors (Actor|GetAllActorsOfClass "BP_Target_C"))
  (for _array_element _outactors
    (CallFunction|ChangeWord _array_element)
    (CallFunction|LoadLetters _array_element)))