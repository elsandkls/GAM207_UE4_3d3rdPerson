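; BP_TemplatePickUp is a configurable pickup actor the player collects into an inventory and can use to add health, energy and mood.
; The construction script applies the custom mesh, thumbnail and texts to its item struct.
; A trigger overlap shows a prompt widget and sets range, letting the character's bound pickup event add the item to the HUD inventory and hide the actor.
; UseAction applies the stat bonuses and destroys it.
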(event OnComponentBeginOverlap(Trigger)
  (params (OverlappedComponent :type Primitive%20Component%20Object%20Reference) (OtherActor :type Actor%20Object%20Reference) (OtherComp :type Primitive%20Component%20Object%20Reference) (OtherBodyIndex :type Integer) (bFromSweep :type Boolean) (SweepResult :type Hit%20Result%20Structure%20%28by%20ref%29))
  ;[1 1 1] Overlap Trigger Script
  (Utilities|Casting|CastToThirdPersonCharacter OtherActor)
  (UserInterface|Viewport|AddtoViewport (Variables|Default|GetPickupTextReference) 0)
  (Variables|Default|SetIsInRange? true))

(event OnComponentEndOverlap(Trigger)
  (params (OverlappedComponent :type Primitive%20Component%20Object%20Reference) (OtherActor :type Actor%20Object%20Reference) (OtherComp :type Primitive%20Component%20Object%20Reference) (OtherBodyIndex :type Integer))
  ;[1 1 1] Overlap Trigger Script
  (Utilities|Casting|CastToThirdPersonCharacter OtherActor)
  (Widget|RemovefromParent (Variables|Default|GetPickupTextReference))
  (Variables|Default|SetIsInRange? false))

(event Custom|PickUp_Event_0
  (bind _characterreference (Variables|Default|GetCharacterReference))
  (bind _bottomhud_object_reference (Variables|/Game/ThirdPersonBP/Blueprints/ThirdPersonCharacter.ThirdPersonCharacter_C|GetBottomHUD_Object_Reference _characterreference))
  ;[1 1 1] Pickup and Add items to inventory to refresh it
  (if (and (Collision|GetActorEnableCollision) (Variables|Default|GetIsInRange?))
    (Utilities|Array|Add (Variables|/Game/Levels/Menus/Bottom_HUD.Bottom_HUD_C|GetInventory _bottomhud_object_reference) (Variables|Default|GetItemInfo))
    (Widget|RemovefromParent (Variables|Default|GetPickupTextReference))
    (Rendering|SetActorHiddenInGame true)
    (Collision|SetActorEnableCollision false)
    (Default|RefreshInventory _bottomhud_object_reference)))

(event Collision|EventActorBeginOverlap
  (params (OtherActor :type Actor%20Object%20Reference)))

(event EventTick
  (params (DeltaSeconds :type Float%20%28single-precision%29)))

(event EventBeginPlay
  (bind _iteminfo (Variables|Default|GetItemInfo))
  (bind (_item _itemthumbnail _pickuptext) (Utilities|Struct|BreakInventoryStructure _iteminfo))
  ;[1 1 1] Event Begin Play
  (bind _returnvalue (UserInterface|CreateWidget "/Game/Levels/Menus/PickupText.PickupText_C"))
  (Variables|Default|SetPickupTextReference _returnvalue)
  (Utilities|Struct|SetmembersinInventoryStructure _iteminfo self)
  (Variables|/Game/Levels/Menus/PickupText.PickupText_C|SetPickupActor (Variables|Default|GetPickupTextReference) _item)
  (Variables|/Game/Levels/Menus/PickupText.PickupText_C|SetPickupText (Variables|Default|GetPickupTextReference) _pickuptext)
  (bind _asthird_person_character (Utilities|Casting|CastToThirdPersonCharacter (Game|GetPlayerCharacter 0)))
  (bind _output_get (Variables|Default|SetCharacterReference _asthird_person_character))
  (EventDispatchers|AssignPickUp _output_get (delegate Custom|PickUp_Event_0)))

(event EventUseAction
  (bind _characterreference (Variables|Default|GetCharacterReference))
  ;[1 1 1] Use Action
  (Variables|/Game/ThirdPersonBP/Blueprints/ThirdPersonCharacter.ThirdPersonCharacter_C|SetHealthValue _characterreference (+ (Variables|/Game/ThirdPersonBP/Blueprints/ThirdPersonCharacter.ThirdPersonCharacter_C|GetHealthValue _characterreference) (Variables|Default|GetAddHealth)))
  (Variables|/Game/ThirdPersonBP/Blueprints/ThirdPersonCharacter.ThirdPersonCharacter_C|SetEnergyValue _characterreference (+ (Variables|/Game/ThirdPersonBP/Blueprints/ThirdPersonCharacter.ThirdPersonCharacter_C|GetEnergyValue _characterreference) (Variables|Default|GetAddEnergy)))
  (Variables|/Game/ThirdPersonBP/Blueprints/ThirdPersonCharacter.ThirdPersonCharacter_C|SetMoodValue _characterreference (+ (Variables|/Game/ThirdPersonBP/Blueprints/ThirdPersonCharacter.ThirdPersonCharacter_C|GetMoodValue _characterreference) (Variables|Default|GetAddMood)))
  (Actor|DestroyActor))

(fn ConstructionScript
  (Utilities|Struct|SetmembersinInventoryStructure (Variables|Default|GetItemInfo) self (Variables|Default|GetCustomImage) (Variables|Default|GetCustomPickupText) (Variables|Default|GetCustomActionText))
  (Components|StaticMesh|SetStaticMesh (Variables|Default|GetStaticMesh) (Variables|Default|GetCustomStaticMesh)))