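; BP_TemplateAmmoPickup is a template ammo pickup with configurable mesh, thumbnail, text and points, packed into an ammo struct.
; BeginPlay creates a prompt widget and binds the pickup event to ThirdPersonCharacter.
; Trigger overlap toggles the prompt and range flag.
; In-range pickup stores the struct, hides the actor, disables collision and refreshes the HUD's ammo inventory, while UseAction destroys the character rather than the pickup.
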(event OnComponentBeginOverlap(Trigger)
  (params (OverlappedComponent :type Primitive%20Component%20Object%20Reference) (OtherActor :type Actor%20Object%20Reference) (OtherComp :type Primitive%20Component%20Object%20Reference) (OtherBodyIndex :type Integer) (bFromSweep :type Boolean) (SweepResult :type Hit%20Result%20Structure%20%28by%20ref%29))
  ;[1 1 1] Overlap Trigger Script
  (Utilities|Casting|CastToThirdPersonCharacter OtherActor)
  (UserInterface|Viewport|AddtoViewport (Variables|Default|GetPickupAmmoTextReference) 0)
  (Variables|Default|SetIsInRange? true))

(event OnComponentEndOverlap(Trigger)
  (params (OverlappedComponent :type Primitive%20Component%20Object%20Reference) (OtherActor :type Actor%20Object%20Reference) (OtherComp :type Primitive%20Component%20Object%20Reference) (OtherBodyIndex :type Integer))
  ;[1 1 1] Overlap Trigger Script
  (Utilities|Casting|CastToThirdPersonCharacter OtherActor)
  (Widget|RemovefromParent (Variables|Default|GetPickupAmmoTextReference))
  (Variables|Default|SetIsInRange? false))

(event Custom|PickUp_Ammo_Event
  ;[1 1 1] Pickup and Add items to inventory to refresh it
  (if (and (Collision|GetActorEnableCollision) (Variables|Default|GetIsInRange?))
    (Utilities|Array|Add (Utilities|Array|MakeArray (Variables|Default|GetReferenceAmmoStruct)) (Variables|Default|GetItemInfo))
    (Widget|RemovefromParent (Variables|Default|GetPickupAmmoTextReference))
    (Rendering|SetActorHiddenInGame true)
    (Collision|SetActorEnableCollision false)
    (Default|RefreshAmmoInventory (Variables|/Game/ThirdPersonBP/Blueprints/ThirdPersonCharacter.ThirdPersonCharacter_C|GetBottomHUD_Object_Reference (Variables|Default|GetCharacterReference)))))

(event Collision|EventActorBeginOverlap
  (params (OtherActor :type Actor%20Object%20Reference)))

(event EventTick
  (params (DeltaSeconds :type Float%20%28single-precision%29)))

(event EventBeginPlay
  (bind _iteminfo (Variables|Default|GetItemInfo))
  (bind (_item _itemthumbnail _pickuptext) (Utilities|Struct|BreakAmmoStructure _iteminfo))
  ;[1 1 1] Event Begin Play
  (bind _returnvalue (UserInterface|CreateWidget "/Game/Levels/Menus/PickupText.PickupText_C"))
  (bind _output_get (Variables|Default|SetPickupAmmoTextReference _returnvalue))
  (Utilities|Struct|SetmembersinAmmoStructure _iteminfo self (Variables|Default|GetCustomImage) (Utilities|Text|ToText(String) (Utilities|String|ToString(Object) _output_get)) (Variables|Default|GetVowel) (Variables|Default|GetPointTotal))
  (Variables|/Game/Levels/Menus/PickupText.PickupText_C|SetPickupActor (Variables|Default|GetPickupAmmoTextReference) _item)
  (Variables|/Game/Levels/Menus/PickupText.PickupText_C|SetPickupText (Variables|Default|GetPickupAmmoTextReference) _pickuptext)
  (bind _asthird_person_character (Utilities|Casting|CastToThirdPersonCharacter (Game|GetPlayerCharacter 0)))
  (bind _output_get_2 (Variables|Default|SetCharacterReference _asthird_person_character))
  (EventDispatchers|AssignPickUp _output_get_2 (delegate Custom|PickUp_Ammo_Event)))

(event EventUseAction
  ;[1 1 1] Use Action
  (Actor|DestroyActor (Variables|Default|GetCharacterReference)))

(fn ConstructionScript
  (Utilities|Struct|SetmembersinAmmoStructure (Variables|Default|GetItemInfo) self (Variables|Default|GetCustomImage) (Variables|Default|GetCustomPickupText) (Variables|Default|GetVowel) (Variables|Default|GetPointTotal))
  (Components|StaticMesh|SetStaticMesh (Variables|Default|GetStaticMesh) (Variables|Default|GetCustomStaticMesh)))